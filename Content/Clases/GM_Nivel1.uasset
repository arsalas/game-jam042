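; Game mode for Level 1 that shows the level's UI and runs a countdown timer.
; On BeginPlay it creates the UI_Level1 widget, stores a reference to it, adds it to the viewport and starts the countdown.
; A custom event re-calls itself after a one-second Delay, decrementing GMTimeL1 while it is above zero, with no action when it runs out.
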(event Custom|CE_timeMinus
  (if (> (Variables|Default|GetGM_TimeL1) 0.0)
    (Utilities|FlowControl|Delay 1.0)
    (Variables|Default|SetGM_TimeL1 (- (Variables|Default|GetGM_TimeL1) 1.0))
    (CallFunction|CETimeMinus)))

(event EventBeginPlay
  (bind _returnvalue (UserInterface|CreateWidget "/Game/Widgets/UI_Level1.UI_Level1_C"))
  (bind _output_get (Variables|Default|SetRef_WL1 _returnvalue))
  (UserInterface|Viewport|AddtoViewport _output_get 0)
  (CallFunction|CETimeMinus))

(fn ConstructionScript)