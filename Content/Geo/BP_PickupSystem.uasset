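; BP_PickupSystem is a prototype pickup actor that shows an input key text prompt when the player overlaps its sphere.
; The overlap enables input on the actor, while any actor end overlap disables it and hides the prompt, as that player check compares the player to itself.
; F destroys the actor; Q calls TestingKeys on ManCharacterLevel2, marked not working with sending to inventory still to do.
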(event OnComponentBeginOverlap(Sphere)
  (params (OverlappedComponent :type Primitive%20Component%20Object%20Reference) (OtherActor :type Actor%20Object%20Reference) (OtherComp :type Primitive%20Component%20Object%20Reference) (OtherBodyIndex :type Integer) (bFromSweep :type Boolean) (SweepResult :type Hit%20Result%20Structure%20%28by%20ref%29))
  (Development|PrintString "Overlapping")
  (if (== OtherActor (Game|GetPlayerCharacter 0))
    (Development|PrintString "Pisando Pickable")
    (Input|EnableInput (Game|GetPlayerController 0))
    ;[1 1 1] Input Key Text Render
    (Rendering|SetVisibility (Variables|Default|GetTextRender_F) true false)))

(event EventBeginPlay)

(event Collision|EventActorBeginOverlap
  (params (OtherActor :type Actor%20Object%20Reference)))

(event EventTick
  (params (DeltaSeconds :type Float%20%28single-precision%29)))

(event Collision|EventActorEndOverlap
  (params (OtherActor :type Actor%20Object%20Reference))
  (if (== (Game|GetPlayerCharacter 0) (Game|GetPlayerCharacter 0))
    (Development|PrintString "No pisando Pickable")
    (Input|DisableInput (Game|GetPlayerController 0))
    ;[1 1 1] Input Key Text Render
    (Rendering|SetVisibility (Variables|Default|GetTextRender_F) false false)))

(event Input|KeyboardEvents|Q
  (params (Key :type Key%20Structure :default "None"))
  ;[1 1 1] Not Working - ToDo : Send To Inventory
  (:Pressed
    (Development|PrintString "Presed Pickup Button")
    (bind _asman_character_level_2 (Utilities|Casting|CastToManCharacterLevel2 (Game|GetPlayerCharacter 0)))
    (Default|TestingKeys _asman_character_level_2)
    (Development|PrintString "Recogida Piedra")))

(event Input|KeyboardEvents|F
  (params (Key :type Key%20Structure :default "None"))
  (:Pressed
    (Actor|DestroyActor)))

(fn ConstructionScript)